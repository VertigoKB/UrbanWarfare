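; Game instance for Urban Warfare that hosts multiplayer servers through an Advanced Sessions node.
; CreateServer creates a session with player slots and LAN option, publishing server name, selected map and language as extra string settings.
; On success it switches on the selected map, though all three cases currently open the PowerPlant level.
; A helper function returns the instance itself.
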(event Custom|CreateServer
  (params (ServerName :type String) (PlayerSlotAmount :type Integer) (Language :type String) (bUseLAN :type Boolean))
  (|AdvancedSession (Utilities|Array|MakeArray (Class|AdvancedSessionsLibrary|MakeLiteralSessionPropertyString "ServerName" ServerName) (Class|AdvancedSessionsLibrary|MakeLiteralSessionPropertyString "ServerMap" (Utilities|String|EnumtoString (Variables|Default|GetSelectedGameMap))) (Class|AdvancedSessionsLibrary|MakeLiteralSessionPropertyString "ServerLanguage" Language)) (Game|GetPlayerController 0) PlayerSlotAmount 0 bUseLAN true false true true true false false false true false true
    (:OnSuccess
      (switch Utilities|FlowControl|Switch|SwitchonE_GameMap (Variables|Default|GetSelectedGameMap)
        (:NewEnumerator0
          _)
        (:NewEnumerator1
          _)
        (:NewEnumerator2
          _))
      (Game|OpenLevel(byObjectReference) "/Game/Level/PowerPlant.PowerPlant"))))

(fn GetGameInstanceRef
  (return self))