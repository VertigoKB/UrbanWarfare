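; Player controller for the main menu that shows and hides the Main Menu, Create Server and Server Browser widgets, opening the Main Menu on BeginPlay.
; A ShowHideWidget event takes a widget selector and a show flag, routing to show or hide functions that switch on the selector.
; Widgets are created lazily on first show, cached in variables for reuse, and removed from parent when hidden.
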(event Custom|ShowHideWidget
  (params (Widget :type E_MainMenuWidget%20Enum :default "NewEnumerator0") (Show :type Boolean))
  (if Show
    (CallFunction|FShowWidget Widget)
    (else
      (CallFunction|FHideWidget Widget))))

(event EventBeginPlay
  (CallFunction|ShowHideWidget "NewEnumerator0" true))

(event EventTick
  (params (DeltaSeconds :type Float%20%28single-precision%29)))

(fn ConstructionScript)

(fn FShowWidget
  (params (Widget :type E_MainMenuWidget%20Enum :default "NewEnumerator0"))
  (switch Utilities|FlowControl|Switch|SwitchonE_MainMenuWidget Widget
    (:NewEnumerator0
      (Variables|Default|GetMainMenu
        (:then
          _)
        (:else
          (bind _returnvalue (UserInterface|CreateWidget "/Game/Blueprints/MainMenu/WB_MainMenu.WB_MainMenu_C"))
          (bind _output_get (Variables|Default|SetMainMenu _returnvalue))))
      (UserInterface|Viewport|AddtoViewport _output_get 0))
    (:NewEnumerator2
      (Variables|Default|GetCreateServer
        (:then
          _)
        (:else
          (bind _returnvalue_2 (UserInterface|CreateWidget "/Game/Blueprints/MainMenu/WB_CreateServer.WB_CreateServer_C"))
          (bind _output_get_2 (Variables|Default|SetCreateServer _returnvalue_2))))
      (UserInterface|Viewport|AddtoViewport _output_get_2 0))
    (:NewEnumerator3
      (Variables|Default|GetServerBrowser
        (:then
          _)
        (:else
          (bind _returnvalue_3 (UserInterface|CreateWidget "/Game/Blueprints/MainMenu/WB_ServerBrowser.WB_ServerBrowser_C"))
          (bind _output_get_3 (Variables|Default|SetServerBrowser _returnvalue_3))))
      (UserInterface|Viewport|AddtoViewport _output_get_3 0))))

(fn FHideWidget
  (params (Widget :type E_MainMenuWidget%20Enum :default "NewEnumerator0"))
  (switch Utilities|FlowControl|Switch|SwitchonE_MainMenuWidget Widget
    (:NewEnumerator0
      (bind _mainmenu (Variables|Default|GetMainMenu)
        (:then
          (Widget|RemovefromParent _mainmenu))
        (:else)))
    (:NewEnumerator2
      (bind _createserver (Variables|Default|GetCreateServer)
        (:then
          (Widget|RemovefromParent _createserver))
        (:else)))
    (:NewEnumerator3
      (bind _serverbrowser (Variables|Default|GetServerBrowser)
        (:then
          (Widget|RemovefromParent _serverbrowser))
        (:else)))))

(fn GetPlayerControllerRef
  (return self))